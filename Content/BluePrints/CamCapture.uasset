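; CamCapture is an actor that tests mapping a PV (photo/video) camera image point to a surface in the world.
; Each tick it turns a point at a quarter of the intrinsics' width and height into a world-space ray from the camera's transform.
; A short Visibility line trace follows that ray, and on a hit draws a debug coordinate system aligned to the surface normal.
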(event `self.ReceiveTick`
  (params (DeltaSeconds :type "Float (single-precision)"))
  (bind (_focallength _width _height) (`HoloLensARFunctionLibrary.GetPVCameraIntrinsics`))
  (bind _returnvalue (`KismetMathLibrary.TransformLocation` (`HoloLensARFunctionLibrary.GetPVCameraToWorldTransform`)))
  (bind (_outhit _returnvalue_2) (`KismetSystemLibrary.LineTraceSingle` _returnvalue (+ _returnvalue (* (`HoloLensARFunctionLibrary.GetWorldSpaceRayFromCameraPoint` (/ (`KismetMathLibrary.MakeVector2D` (`KismetMathLibrary.Conv_IntToDouble` _width) (`KismetMathLibrary.Conv_IntToDouble` _height)) 4.0)) 200.0)) "TraceTypeQuery1"))
  (if _returnvalue_2
    (bind (_bblockinghit _binitialoverlap _time _distance _location _impactpoint _normal) (`GameplayStatics.BreakHitResult` _outhit))
    (`KismetSystemLibrary.DrawDebugCoordinateSystem` _location (`KismetMathLibrary.Conv_VectorToRotator` _normal))))

(fn `UserConstructionScript`)