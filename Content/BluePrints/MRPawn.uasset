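; MRPawn is a mixed reality pawn that sets up hand interaction and spawns chess king pieces on input.
; BeginPlay spawns two UXT hand interaction actors, one per hand, with near cursors shown on grab targets.
; The GenerateWhiteKing input action spawns a scaled-down WhiteKing at the pawn's location and prints a debug string.
; The tracked-geometry event is empty; logic applying an orange wireframe material to world meshes is left disconnected.
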(event `self.ReceiveBeginPlay`
  (bind _returnvalue (`KismetMathLibrary.MakeTransform` (0.0 0.0 0.0)))
  (`|SpawnActorFromClass` "/Script/UXTools.UxtHandInteractionActor" _returnvalue "AlwaysSpawn" "OverrideRootScale" self true "Left" null)
  (`|SpawnActorFromClass` "/Script/UXTools.UxtHandInteractionActor" _returnvalue "AlwaysSpawn" "OverrideRootScale" self true "Right" null))

(event `InputAction|GenerateWhiteKing`
  (params (Key :type "Key Structure"))
  (:`Pressed`
    (`|SpawnActorFromClass` "/Game/BluePrints/WhiteKing.WhiteKing_C" (`KismetMathLibrary.MakeTransform` (`self.K2_GetActorLocation`) (struct) (0.05 0.05 0.05)) "AdjustIfPossibleButAlwaysSpawn" "OverrideRootScale" null null)
    (`KismetSystemLibrary.PrintString` "GenerateWhiteKing")))

(event `self.ARTrackableNotify.OnUpdateTrackedGeometry`
  (params (TrackedGeometry :type "ARTrackedGeometry Object Reference")))

(fn `UserConstructionScript`)